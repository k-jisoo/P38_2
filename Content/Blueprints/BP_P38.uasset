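; BP_P38 is a player-controllable P-38 aircraft pawn that constantly moves along its forward vector.
; Roll and pitch axes apply frame-rate-scaled local rotation, while the Boost action switches movement input between full and half strength.
; On BeginPlay it registers the Right and Left components, likely propellers, with BPRotatingSceneComponent to spin about X.
; A separate RotatePropeller helper exists but is not called in these graphs.
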(event `self.ReceiveBeginPlay`
  (`/Game/Blueprints/BP_RotatingStaticMesh_1.AddSceneComponent` (`self.BP_RotatingSceneComponent`) (`self.Right`))
  (`/Game/Blueprints/BP_RotatingStaticMesh_1.AddSceneComponent` (`self.BP_RotatingSceneComponent`) (`self.Left`))
  (set `/Game/Blueprints/BP_RotatingStaticMesh_1.Axis` (struct :`Roll` 1.0) (`self.BP_RotatingSceneComponent`)))

(event `self.ReceiveTick`
  (params (DeltaSeconds :type "Float (single-precision)"))
  (`self.AddMovementInput` (`self.GetActorForwardVector`) (`self.Boost`)))

(event `InputAxis|Roll`
  (params (AxisValue :type "Float (single-precision)"))
  ;[1 1 1] Roll
  (`self.K2_AddActorLocalRotation` (`KismetMathLibrary.MakeRotator` (* AxisValue (`self.RotationSpeed`) (`GameplayStatics.GetWorldDeltaSeconds`)))))

(event `InputAction|Boost`
  (params (Key :type "Key Structure"))
  (:`Pressed`
    (set `self.Boost` 1.0))
  (:`Released`
    (set `self.Boost` 0.5)))

(event `InputAxis|Pitch`
  (params (AxisValue :type "Float (single-precision)"))
  ;[1 1 1] Pitch
  (`self.K2_AddActorLocalRotation` (`KismetMathLibrary.MakeRotator` 0.0 (* AxisValue (`self.RotationSpeed`) (`GameplayStatics.GetWorldDeltaSeconds`)))))

(fn `RotatePropeller`
  (params (Where :type "SceneComponent Object Reference"))
  (`SceneComponent.K2_AddLocalRotation` Where (`KismetMathLibrary.MakeRotator` (* (`GameplayStatics.GetWorldDeltaSeconds`) (`self.Speed`))) false false))

(fn `UserConstructionScript`)